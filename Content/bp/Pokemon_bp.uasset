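; Wild Pokémon encounter trigger that opens a battle screen when the Hero overlaps its Box.
; It picks a random ID from WildPokemonID, reads that row from the Wild_pokemon_datas table, randomizes level around the base and scales HP by level.
; It clears all widgets, then creates Battle_UI with the enemy's stats and the player's items and Pokémon from the save game.
; Without a valid save, it only prints a debug message.
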(event OnComponentBeginOverlap(Box)
  (params (OverlappedComponent :type Primitive%20Component%20Object%20Reference) (OtherActor :type Actor%20Object%20Reference) (OtherComp :type Primitive%20Component%20Object%20Reference) (OtherBodyIndex :type Integer) (bFromSweep :type Boolean) (SweepResult :type Hit%20Result%20Structure%20%28by%20ref%29))
  (Utilities|Casting|CastToHero OtherActor)
  (Utilities|IsValid (Variables|Default|GetWildPokemon_UI)
    (:Is%20Valid
      _)
    (:Is%20Not%20Valid
      _))
  (Viewport|RemoveAllWidgets)
  (bind _outrownames (DataTable|GetDataTableRowNames "/Game/Data/wild_pokemon_datas.wild_pokemon_datas"))
  (bind _returnvalue (Utilities|GetDataTableRow "/Game/Data/wild_pokemon_datas.wild_pokemon_datas" (Utilities|Array|Get(acopy) _outrownames (- (Utilities|Array|Get(acopy) (Variables|Default|GetWildPokemon_ID) (Math|Random|RandomIntegerinRange 0 (- (Utilities|Array|Length (Variables|Default|GetWildPokemon_ID)) 1))) 1)))
    (:then
      (bind _output_get (Variables|Default|SetWildPokemon_level (+ (.pokemon_level (Utilities|Struct|Breakpokemon_structure _returnvalue)) (Math|Random|RandomIntegerinRange -2 2))))
      ;[1 1 1] load savefiles into game
      (bind _returnvalue_2 (SaveGame|DoesSaveGameExist (Variables|Default|Getsave%20Game%20Slot)))
      (if _returnvalue_2
        (Development|PrintString "exist slot")
        (bind _returnvalue_3 (SaveGame|LoadGamefromSlot (Variables|Default|Getsave%20Game%20Slot)))
        (bind _asmy_save_game (Utilities|Casting|CastTomy_save_game _returnvalue_3)
          (:then
            (bind _output_get_2 (Variables|Default|SetSave%202 _asmy_save_game))
            (bind _returnvalue_4 (UserInterface|CreateWidget "/Game/GUI/Battle_UI.Battle_UI_C" 0 (.pokemon_ID (Utilities|Struct|Breakpokemon_structure _returnvalue)) (Math|Random|RandomBool) (.pokemon_Name (Utilities|Struct|Breakpokemon_structure _returnvalue)) _output_get (Math|Conversions|ToFloat(Integer) (* (.Pokemon_HP (Utilities|Struct|Breakpokemon_structure _returnvalue)) _output_get)) (Math|Conversions|ToFloat(Integer) (* (.Pokemon_HP (Utilities|Struct|Breakpokemon_structure _returnvalue)) _output_get)) (.Pokemon_initAttack (Utilities|Struct|Breakpokemon_structure _returnvalue)) (.Pokemon_Ability (Utilities|Struct|Breakpokemon_structure _returnvalue)) (.pokemon_front_asEnemy (Utilities|Struct|Breakpokemon_structure _returnvalue)) (Variables|/Game/savegame/my_save_game.my_save_game_C|GetS_ball _output_get_2) (Variables|/Game/savegame/my_save_game.my_save_game_C|GetS_coin _output_get_2) (Variables|/Game/savegame/my_save_game.my_save_game_C|GetS_medicine _output_get_2) (Variables|/Game/savegame/my_save_game.my_save_game_C|GetS_pokemon_Structure _output_get_2)))
            (bind _output_get_3 (Variables|Default|SetWildPokemon_UI _returnvalue_4))
            (UserInterface|Viewport|AddtoViewport _output_get_3 0))
          (:CastFailed
            (Development|PrintString "cast fail")))
        (else
          (Development|PrintString "no exist slot"))))))

(fn ConstructionScript)